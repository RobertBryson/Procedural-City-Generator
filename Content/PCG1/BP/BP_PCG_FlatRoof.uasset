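; Custom PCG Blueprint node "FlatRoof" that builds a flat roof mesh from input points so it lines up with the building.
; A point loop collects each point's location, offset by ActorLocation and nudged slightly down, as polygon vertices.
; Geometry Script triangulates that polygon on a pooled compute mesh and simplifies it to planar.
; The result is wrapped with a material as PCG dynamic mesh data and output on the FlatRoof pin.
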(fn ExecutewithContext
  (params (InContext :type PCG%20Context%20Structure%20%28by%20ref%29) (Input :type PCG%20Data%20Collection%20Structure%20%28by%20ref%29))
  (Utilities|FlowControl|Sequence
    (:then_0
      ;[0.15 0.15 0.15 0.5] Gets points data, exits if none
      (bind _aspcgpoint_data (Utilities|Casting|CastToPCGPointData (.Data (PCG|TaggedData|BreakTaggedData (Utilities|Array|Get(acopy) (.taggeddata Input)))))
        (:then
          (Variables|Default|SetAs%20PCGPoint%20Data _aspcgpoint_data))
        (:CastFailed
          (return ""))))
    (:then_1
      ;[0.15 0.15 0.15 0.5] Gets the position of each point and adds to FlatRoofPos array
      (PCG|FlowControl|PointLoop InContext (Variables|Default|GetAs%20PCGPoint%20Data) 0)
      (bind _returnvalue (Class|GeometryScriptLibraryMeshPoolFunctions|GetGlobalMeshPool))
      ;[0.15 0.15 0.15 0.5] Create mesh and set points to line up with building points
      (bind _mesh (Utilities|RequestandReleaseComputeMesh _returnvalue)
        (:With%20Mesh
          (LocalVariables|SetCreatedMesh _mesh)
          (bind _returnvalue_2 (Class|GeometryScriptLibraryMeshPrimitiveFunctions|AppendTriangulatedPolygon3D (LocalVariables|GetCreatedMesh) (Utilities|Struct|MakeGeometryScriptPrimitiveOptions "SingleGroup" false "Uniform" 0) (Math|Transform|MakeTransform "0, 0, 0" "0, 0, 0" "1.000000,1.000000,1.000000") (Variables|Default|GetFlatRoofPos)))
          (Class|GeometryScriptLibraryMeshSimplifyFunctions|ApplySimplifytoPlanar _returnvalue_2 (Utilities|Struct|MakeGeometryScriptPlanarSimplifyOptions 2.0 true))
          ;[1 1 1] construct dynamic mesh data
          (bind _returnvalue_3 (Game|ConstructObjectfromClass "/Script/PCG.PCGDynamicMeshData"))
          (bind _output_get (LocalVariables|SetConstructedMesh _returnvalue_3))
          (Initialization|Initialize _output_get (LocalVariables|GetCreatedMesh) (Utilities|Array|MakeArray (Variables|Default|Getmaterial)) false)
          (Class|GeometryScriptLibraryMeshPoolFunctions|DiscardGlobalMeshPool)
          (return (Utilities|Struct|MakePCGDataCollection (Utilities|Array|MakeArray (PCG|TaggedData|MakeTaggedData (LocalVariables|GetConstructedMesh) 0 "FlatRoof")) true)))))))

(fn PointLoopBody
  (params (InContext :type PCG%20Context%20Structure%20%28by%20ref%29) (InData :type PCG%20Point%20Data%20Object%20Reference) (InPoint :type PCG%20Point%20Structure%20%28by%20ref%29) (OutMetadata :type PCG%20Metadata%20Object%20Reference) (Iteration :type Integer64))
  (Utilities|Array|Add (Variables|Default|GetFlatRoofPos) (+ (.Location (Math|Transform|BreakTransform (.Transform (Utilities|Struct|BreakPCGPoint InPoint)))) (Variables|Default|GetActorLocation) "0.000000,0.000000,-1.000000"))
  (return "" false))

(fn NodeTitleOverride
  (return "FlatRoof"))