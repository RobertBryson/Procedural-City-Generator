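; BP_TOWN is a PCG town actor with a BuildingGenerator and a randomized OuterCitySpline boundary.
; SetSpline rebuilds the spline with four world-space points, one per quadrant around the world origin, at random offsets between MinSplineDist and MaxSplineDist.
; Generate and Clean both only call Cleanup on BuildingGenerator, so Generate triggers no generation here.
; A MarkPropertyDirty node is left unconnected, and the construction script is empty.
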(event Custom|Generate
  (Class|PCGComponent|Cleanup (Variables|Default|GetBuildingGenerator) true))

(event Custom|Clean
  (Class|PCGComponent|Cleanup (Variables|Default|GetBuildingGenerator) true))

(event Custom|SetSpline
  (Spline|ClearSplinePoints (Variables|Default|GetOuterCitySpline) false)
  (Spline|AddSplinePoint (Variables|Default|GetOuterCitySpline) (Math|Vector|MakeVector (Math|Random|RandomFloatinRange (Variables|Default|GetMinSplineDist) (Variables|Default|GetMaxSplineDist)) (Math|Random|RandomFloatinRange (Variables|Default|GetMinSplineDist) (Variables|Default|GetMaxSplineDist)) 0.0) "World" false)
  (Spline|AddSplinePoint (Variables|Default|GetOuterCitySpline) (Math|Vector|MakeVector (Math|Random|RandomFloatinRange (* (Variables|Default|GetMinSplineDist) -1.0) (* (Variables|Default|GetMaxSplineDist) -1.0)) (Math|Random|RandomFloatinRange (Variables|Default|GetMinSplineDist) (Variables|Default|GetMaxSplineDist)) 0.0) "World" false)
  (Spline|AddSplinePoint (Variables|Default|GetOuterCitySpline) (Math|Vector|MakeVector (Math|Random|RandomFloatinRange (* (Variables|Default|GetMinSplineDist) -1.0) (* (Variables|Default|GetMaxSplineDist) -1.0)) (Math|Random|RandomFloatinRange (* (Variables|Default|GetMinSplineDist) -1.0) (* (Variables|Default|GetMaxSplineDist) -1.0)) 0.0) "World" false)
  (Spline|AddSplinePoint (Variables|Default|GetOuterCitySpline) (Math|Vector|MakeVector (Math|Random|RandomFloatinRange (Variables|Default|GetMinSplineDist) (Variables|Default|GetMaxSplineDist)) (Math|Random|RandomFloatinRange (* (Variables|Default|GetMinSplineDist) -1.0) (* (Variables|Default|GetMaxSplineDist) -1.0)) 0.0) "World" true))

(fn ConstructionScript)